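; BP_Cell is an interactable slot in the second mini-game that receives a BP_Letter carried by the player.
; On Interact, it checks the BP_Player hand for a grabbed letter, releases it and passes it to PlaceLetter.
; PlaceLetter safely disables the letter's physics, snaps and welds it to LetterCell at world scale, and stores it as PlacedActor.
; CanInteract always returns true, with no check for an already filled cell.
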(event EventBeginPlay)

(fn ConstructionScript)

(fn PlaceLetter
  (params (Letter :type BP%20Letter%20Object%20Reference))
  (Utilities|IsValid Letter
    (:Is%20Valid
      (CallFunction|SafeDisablePhys Letter)
      (Transformation|AttachComponentToComponent Letter (Variables|Default|GetLetterCell) "None" "SnapToTarget" "SnapToTarget" "KeepWorld" true)
      (Variables|Default|SetPlacedActor Letter))))

(fn CanInteract
  (return true))

(fn Interact
  (params (PlayerController :type Player%20Controller%20Object%20Reference))
  (bind _asbp_player (Utilities|Casting|CastToBP_Player (Pawn|GetControlledPawn PlayerController)))
  (Utilities|IsValid (Default|GetHand _asbp_player)
    (:Is%20Valid
      (if (.HasGrabbed (Default|GetGrabbedActor (Default|GetHand _asbp_player)))
        (if (.bSuccess (Utilities|Casting|CastToBP_Letter (.GrabbedActor (Default|GetGrabbedActor (Default|GetHand _asbp_player)))))
          (bind _releasedactor (Default|Release (Default|GetHand _asbp_player)))
          (bind _asbp_letter (Utilities|Casting|CastToBP_Letter _releasedactor))
          (CallFunction|PlaceLetter _asbp_letter)
          (return))))))