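; BP_SpawnerController spawns a random number of actors of a configured class at a random selection of its target spawner locations on BeginPlay.
; Spawn picks a count between the min and max, shuffles the Targets array, and always spawns at the first targets' transforms.
; The construction script takes ownership of the targets and clamps the minimum count, while ShowConnections draws debug links to them.
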(event Custom|ShowConnections
  ;[0.1094 0.3085 1] Debug
  (Rendering|Debug|FlushPersistentDebugLines)
  (CallFunction|ShowConnect self (Variables|Default|GetTargets) "(R=1.000000,G=1.000000,B=1.000000,A=1.000000)"))

(event EventBeginPlay
  (CallFunction|Spawn))

(fn ConstructionScript
  (for _array_element (Variables|Default|GetTargets)
    (Actor|SetOwner _array_element self))
  (Variables|Default|SetMinSpawnCount (Math|Integer|Clamp(Integer) (Variables|Default|GetMinSpawnCount) 0 (Variables|Default|GetMaxSpawnCount))))

(fn Spawn
  (bind _targets (Variables|Default|GetTargets))
  (Variables|Default|SetSpawnCount (Math|Random|RandomIntegerinRange (Variables|Default|GetMinSpawnCount) (Variables|Default|GetMaxSpawnCount)))
  (Utilities|Array|Shuffle _targets)
  (bind (_array_element _array_index) (Utilities|Array|ForEachLoopwithBreak _targets :!label _label)
    (:LoopBody
      (if (< _array_index (Variables|Default|GetSpawnCount))
        (Game|SpawnActorfromClass (Variables|Default|GetSpawnClass) (Transformation|GetActorTransform _array_element) "AlwaysSpawn" 0 0)
        (else
          (goto _label Break))))))

(fn HaveSpawner
  (params (Spawner :type BP%20Item%20Spawner%20Object%20Reference))
  (return (>= (Utilities|Array|FindItem (Variables|Default|GetTargets) Spawner) 0)))