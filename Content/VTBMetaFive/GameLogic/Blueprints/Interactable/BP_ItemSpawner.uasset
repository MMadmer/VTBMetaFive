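; BP_ItemSpawner is an interactable spawner point that belongs to a BP_SpawnerController through actor ownership.
; On BeginPlay it reassigns its owner to the owner's owner if the controller does not list it as a spawner, then destroys itself if no valid owner remains.
; A debug event draws a connection line from the spawner to its owner.
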(event Custom|ShowConnections
  ;[0.1667 0.3425 1] Debug
  (Rendering|Debug|FlushPersistentDebugLines)
  (CallFunction|ShowConnect self (Utilities|Array|MakeArray (Components|GetOwner)) "(R=1.000000,G=1.000000,B=1.000000,A=1.000000)"))

(event EventBeginPlay
  (CallFunction|UpdateOwner)
  (Utilities|IsValid (Components|GetOwner)
    (:Is%20Not%20Valid
      (Actor|DestroyActor))))

(fn ConstructionScript)

(fn UpdateOwner
  (bind _asbp_spawner_controller (Utilities|Casting|CastToBP_SpawnerController (Components|GetOwner)))
  (if (not (Default|HaveSpawner _asbp_spawner_controller self))
    (Actor|SetOwner (Components|GetOwner (Components|GetOwner)))))