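; Global Blueprint function library with helpers for radius-based actor queries and smooth timer math.
; GetActorsInRadius adds a temporary sphere component to the given actor, collects overlapping actors whose exact class is in the filter list, then destroys the sphere.
; CalcSmoothTimer converts a duration and frame rate into a per-tick delay and normalized progress step.
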(fn GetActorsinRadius
  (params (MainActor :type Actor%20Object%20Reference) (Radius :type Float%20%28single-precision%29) (Filter :type Array%20of%20Actor%20Class%20References))
  (bind _returnvalue (Game|AddComponentbyClass MainActor "/Script/Engine.SphereComponent" false))
  (Components|Sphere|SetSphereRadius _returnvalue Radius true)
  (for _array_element (Collision|GetOverlappingActors _returnvalue 0 :!class /Script/Engine.PrimitiveComponent)
    (if (>= (Utilities|Array|FindItem Filter (Utilities|GetClass _array_element)) 0)
      (Utilities|Array|Add (LocalVariables|GetFinalActors) _array_element)))
  (Components|DestroyComponent _returnvalue)
  (return (LocalVariables|GetFinalActors)))

(fn CalcSmoothTimer
  (params (Time :type Float%20%28single-precision%29) (FrameRate :type Integer))
  (bind _returnvalue (Math|Conversions|ToFloat(Integer) FrameRate))
  (return (/ 1.0 _returnvalue) (/ 1.0 (* Time _returnvalue))))