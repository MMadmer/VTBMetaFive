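; BP_Letter is a physical letter level object for the first mini-game, showing one letter mesh picked from a letter-to-mesh table.
; The construction script previews the chosen SetLetter mesh in the editor.
; On BeginPlay, ApplyMesh picks a random entry or the matching SetLetter, stores it as CurrentLetter, and overrides the mesh's mass.
; GetLetter exposes the current letter to other objects.
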(event EventBeginPlay
  (CallFunction|ApplyMesh)
  (Class|PrimitiveComponent|SetMassOverrideinKg (Variables|Default|GetSM_Letter) "None" (Variables|Default|GetMass) true))

(fn ConstructionScript
  (bind _array_element (Utilities|Array|ForEachLoopwithBreak (Variables|Default|GetLetters) :!label _label)
    (:LoopBody
      (if (Utilities|Enum|Equal(Enum) (.Letter (Utilities|Struct|BreakF_LetterInfo _array_element)) (Variables|Default|GetSetLetter))
        (Components|StaticMesh|SetStaticMesh (Variables|Default|GetSM_Letter) (.Mesh (Utilities|Struct|BreakF_LetterInfo _array_element)))
        (goto _label Break)))))

(fn GetLetter
  (return (.letter (Variables|Default|GetCurrentLetter))))

(fn ApplyMesh
  (if (Variables|Default|GetRandomLetter)
    (bind _output_get (Variables|Default|SetCurrentLetter (.OutItem (Utilities|Array|Random (Variables|Default|GetLetters)))))
    (Components|StaticMesh|SetStaticMesh (Variables|Default|GetSM_Letter) (.mesh _output_get))
    (else
      (bind _array_element (Utilities|Array|ForEachLoopwithBreak (Variables|Default|GetLetters) :!label _label)
        (:LoopBody
          (if (Utilities|Enum|Equal(Enum) (.Letter (Utilities|Struct|BreakF_LetterInfo _array_element)) (Variables|Default|GetSetLetter))
            (Variables|Default|SetCurrentLetter _array_element)
            (Components|StaticMesh|SetStaticMesh (Variables|Default|GetSM_Letter) (.Mesh (Utilities|Struct|BreakF_LetterInfo _array_element)))
            (goto _label Break)))))))