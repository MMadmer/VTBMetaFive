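; BP_Cell is an interactable letter slot for the first minigame, where the player places and retrieves BP_Letter actors.
; Interact releases a letter held in the player's hand into PlaceLetter, or hands the stored letter back to an empty hand.
; PlaceLetter disables physics, snaps the letter to LetterPlace, strips its "grab" tag until retrieval and fires OnLetterPlaced.
; Placement does not check whether the cell is already filled, and its own OnPlacement handler is empty.
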(event Custom|OnPlacement)

(event EventBeginPlay
  (EventDispatchers|AssignOnLetterPlaced (delegate Custom|OnPlacement)))

(fn ConstructionScript)

(fn PlaceLetter
  (params (Letter :type BP%20Letter%20Object%20Reference))
  (Utilities|IsValid Letter
    (:Is%20Valid
      (bind _asprimitive_component (Utilities|Casting|CastToPrimitiveComponent (Variables|/Script/Engine.Actor|GetRootComponent Letter)))
      (Physics|SetSimulatePhysics _asprimitive_component false)
      (Transformation|AttachComponentToComponent Letter (Variables|Default|GetLetterPlace) "None" "SnapToTarget" "SnapToTarget" "KeepWorld" true)
      (Variables|Default|SetPlacedActor Letter)
      (Variables|Default|SetHasPlased true)
      (Utilities|Array|RemoveItem (Variables|/Script/Engine.Actor|GetTags (Variables|Default|GetPlacedActor)) "grab")
      (Default|CallOnLetterPlaced))))

(fn CanInteract
  (return true))

(fn Interact
  (params (Pawn :type Pawn%20Object%20Reference))
  (bind _asbp_player (Utilities|Casting|CastToBP_Player Pawn))
  (Utilities|IsValid (Default|GetHand _asbp_player)
    (:Is%20Valid
      (if (.HasGrabbed (Default|GetGrabbedActor (Default|GetHand _asbp_player)))
        (if (.bSuccess (Utilities|Casting|CastToBP_Letter (.GrabbedActor (Default|GetGrabbedActor (Default|GetHand _asbp_player)))))
          (bind _releasedactor (Default|Release (Default|GetHand _asbp_player)))
          (bind _asbp_letter (Utilities|Casting|CastToBP_Letter _releasedactor))
          (CallFunction|PlaceLetter _asbp_letter)
          (return))
        (elif (Variables|Default|GetHasPlased)
          (Utilities|Array|AddUnique (Variables|/Script/Engine.Actor|GetTags (Variables|Default|GetPlacedActor)) "grab")
          (Default|Grab (Default|GetHand _asbp_player) (Variables|Default|GetPlacedActor))
          (Variables|Default|SetHasPlased false))))))