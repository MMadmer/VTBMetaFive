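; Word puzzle controller that checks letters placed into a row of target cells against a target word.
; With AutoActivate, it picks a random AllWords key on BeginPlay, enables enough cells for it and sends the paired text to billboards.
; Cell place/remove events update CurrentWord by cell index; once full, it fires word-complete or wrong-word.
; It destroys itself without cells and has a debug event drawing cell connections.
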(event Custom|OnLetterPlaced
  (params (Cell :type BP%20Cell%20Object%20Reference) (Letter :type String))
  (bind _targetcells (Variables|Default|GetTargetCells))
  (bind _returnvalue (Utilities|Array|FindItem _targetcells Cell))
  (if (>= _returnvalue 0)
    (Utilities|Array|SetArrayElem (Variables|Default|GetCurrentWord) _returnvalue Letter)
    (if (CallFunction|WordCollected)
      (if (CallFunction|CheckWord)
        (Default|CallOnWordComplete)
        (else
          (Default|CallOnWrongWord))))))

(event Custom|OnLetterRemoved
  (params (Cell :type BP%20Cell%20Object%20Reference))
  (bind _targetcells (Variables|Default|GetTargetCells))
  (bind _returnvalue (Utilities|Array|FindItem _targetcells Cell))
  (if (>= _returnvalue 0)
    (Utilities|Array|SetArrayElem (Variables|Default|GetCurrentWord) _returnvalue "")))

(event Custom|ShowConnections
  ;[0.1771 0.3419 1] Debug
  (Rendering|Debug|FlushPersistentDebugLines)
  (CallFunction|ShowConnect self (Variables|Default|GetTargetCells) "(R=0.000000,G=0.400142,B=1.000000,A=1.000000)"))

(event EventBeginPlay
  (if (!= (Utilities|Array|Length (Variables|Default|GetTargetCells)) 0)
    (for _array_element (Variables|Default|GetTargetCells)
      (EventDispatchers|AssignOnLetterPlaced _array_element (delegate Custom|OnLetterPlaced))
      (EventDispatchers|AssignOnLetterRemoved _array_element (delegate Custom|OnLetterRemoved)))
    (if (Variables|Default|GetAutoActivate)
      (CallFunction|GenerateWord))
    (else
      (Actor|DestroyActor))))

(fn ConstructionScript)

(fn SetWord
  (params (NewWord :type String))
  (bind _output_get (Variables|Default|SetTargetWord (Utilities|String|GetCharacterArrayfromString (Utilities|String|ToLower NewWord))))
  (bind _output_get_2 (Variables|Default|SetCurrentWord _output_get))
  (for _index (range 0 (- (Utilities|Array|Length _output_get_2) 1))
    (Utilities|Array|SetArrayElem (Variables|Default|GetCurrentWord) _index ""))
  (for (_array_element _array_index) (Variables|Default|GetTargetCells)
    (Class|BPILevelTools|Activate(Message) _array_element)
    (if (not (Utilities|Array|IsValidIndex (Variables|Default|GetTargetWord) _array_index))
      (Class|BPILevelTools|Deactivate(Message) _array_element))))

(fn CheckWord
  (return (Utilities|Enum|Equal(Enum) (Utilities|String|JoinStringArray (Variables|Default|GetCurrentWord) "") (Utilities|String|JoinStringArray (Variables|Default|GetTargetWord) ""))))

(fn WordCollected
  (bind _array_element (Utilities|Array|ForEachLoopwithBreak (Variables|Default|GetCurrentWord) :!label _label)
    (:LoopBody
      (if (Utilities|Enum|Equal(Enum) _array_element "")
        (LocalVariables|SetHasNone true)
        (goto _label Break)))
    (:Completed
      (return (not (LocalVariables|GetHasNone))))))

(fn GenerateWord
  (bind _keys (Utilities|Map|Keys (Variables|Default|GetAllWords)))
  (if (>= (Utilities|Array|Length _keys) 0)
    (LocalVariables|SetNewWord (.OutItem (Utilities|Array|Random _keys)))
    (LocalVariables|SetNewText (.Value (Utilities|Map|Find (Variables|Default|GetAllWords) (LocalVariables|GetNewWord))))
    (CallFunction|SetWord (LocalVariables|GetNewWord))
    (for _array_element (Variables|Default|GetBilboardsToView)
      (Class|BPIUI|SendText(Message) _array_element (LocalVariables|GetNewText)))))