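; BP_SpawnerController is a level object that spawns a random number of SpawnClass actors, between min and max counts, across its linked Targets.
; Spawn picks a random target for each actor, so points can repeat, and runs on BeginPlay when AutoActivate is set.
; The construction script makes itself each target's owner and clamps the minimum count.
; HaveSpawner checks target membership, and ShowConnections draws debug links to the targets.
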(event Custom|ShowConnections
  ;[0.1094 0.3085 1] Debug
  (Rendering|Debug|FlushPersistentDebugLines)
  (CallFunction|ShowConnect self (Variables|Default|GetTargets) "(R=1.000000,G=1.000000,B=1.000000,A=1.000000)"))

(event EventBeginPlay
  (if (Variables|Default|GetAutoActivate)
    (CallFunction|Spawn)))

(fn ConstructionScript
  (for _array_element (Variables|Default|GetTargets)
    (Actor|SetOwner _array_element self))
  (Variables|Default|SetMinSpawnCount (Math|Integer|Clamp(Integer) (Variables|Default|GetMinSpawnCount) 0 (Variables|Default|GetMaxSpawnCount))))

(fn Spawn
  (LocalVariables|SetSpawnCount (Math|Random|RandomIntegerinRange (Variables|Default|GetMinSpawnCount) (Variables|Default|GetMaxSpawnCount)))
  (while (> (LocalVariables|GetSpawnCount) 0)
    (Game|SpawnActorfromClass (Variables|Default|GetSpawnClass) (Transformation|GetActorTransform (.OutItem (Utilities|Array|Random (Variables|Default|GetTargets)))) "AlwaysSpawn" 0 0)
    (Math|Integer|DecrementInt (LocalVariables|GetSpawnCount))))

(fn HaveSpawner
  (params (Spawner :type BP%20Item%20Spawner%20Object%20Reference))
  (return (>= (Utilities|Array|FindItem (Variables|Default|GetTargets) Spawner) 0)))