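; BP_Bilboard is a level billboard that shows an image and text on a widget and can be raised and lowered.
; On BeginPlay it passes BackImage to the MainWidget's widget, and SendText forwards text to the same widget.
; Activate plays the Activation timeline, whose Open track scaled by OpenHeight sets the relative Z of SMBilboard, and Deactivate reverses that timeline.
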(event EventBeginPlay
  (Class|BPIUI|SetImage(Message) (UserInterface|GetWidget (Variables|Default|GetMainWidget)) (Variables|Default|GetBackImage)))

(event EventActivate
  (bind _sm_bilboard (Variables|Default|GetSM_Bilboard))
  (bind _relativelocation (Variables|/Script/Engine.SceneComponent|GetRelativeLocation _sm_bilboard))
  (bind _open (Timeline|Activation Play)
    (:Update
      (Transformation|SetRelativeLocation _sm_bilboard (Math|Vector|MakeVector (.x _relativelocation) (.y _relativelocation) (* _open (Variables|Default|GetOpenHeight))) false false))))

(event EventDeactivate
  (bind _sm_bilboard (Variables|Default|GetSM_Bilboard))
  (bind _relativelocation (Variables|/Script/Engine.SceneComponent|GetRelativeLocation _sm_bilboard))
  (bind _open (Timeline|Activation Reverse)
    (:Update
      (Transformation|SetRelativeLocation _sm_bilboard (Math|Vector|MakeVector (.x _relativelocation) (.y _relativelocation) (* _open (Variables|Default|GetOpenHeight))) false false))))

(event EventSendText
  (params (Text :type Text))
  (Class|BPIUI|SendText(Message) (UserInterface|GetWidget (Variables|Default|GetMainWidget)) Text))

(fn ConstructionScript)