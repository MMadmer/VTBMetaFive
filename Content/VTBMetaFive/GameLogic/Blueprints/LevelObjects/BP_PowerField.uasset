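; BP_PowerField is a level object that forms a box field and reacts to grabbed objects of prohibited classes.
; The construction script sizes a blocking box and an overlap box from a shared Extend value.
; When an overlapping actor's class is in ProhibitedClasses and it carries the "grabbed" tag, the field calls TryThrowMessage on that actor's owner.
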(event OnComponentBeginOverlap(OverlappingBox)
  (params (OverlappedComponent :type Primitive%20Component%20Object%20Reference) (OtherActor :type Actor%20Object%20Reference) (OtherComp :type Primitive%20Component%20Object%20Reference) (OtherBodyIndex :type Integer) (bFromSweep :type Boolean) (SweepResult :type Hit%20Result%20Structure%20%28by%20ref%29))
  (if (>= (Utilities|Array|FindItem (Variables|Default|GetProhibitedClasses) (Utilities|GetClass OtherActor)) 0)
    (if (>= (Utilities|Array|FindItem (Variables|/Script/Engine.Actor|GetTags OtherActor) "grabbed") 0)
      (Class|BPIPlayerControls|TryThrow(Message) (Components|GetOwner OtherActor)))))

(event EventBeginPlay)

(fn ConstructionScript
  (bind _extend (Variables|Default|GetExtend))
  (Components|Box|SetBoxExtent (Variables|Default|GetBlockingBox) _extend true)
  (Components|Box|SetBoxExtent (Variables|Default|GetOverlappingBox) _extend true))