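; BP_PlayerState is a player state Blueprint that holds the player's money balance and the functions to read and change it.
; SetMoney clamps the balance between zero and a fixed cap, and both GiveMoney and TakeMoney write through it.
; Give and take ignore non-positive amounts, and TakeMoney deducts only when funds suffice, returning whether it succeeded.
; The event graph and construction script contain no logic.
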(event EventBeginPlay)

(fn ConstructionScript)

(fn SetMoney
  (params (Count :type Integer))
  (Variables|Default|SetMoney (Math|Integer|Clamp(Integer) Count 0 999999999)))

(fn GiveMoney
  (params (Count :type Integer))
  (if (> Count 0)
    (Money|SetMoney (+ (Variables|Default|GetMoney) Count))))

(fn TakeMoney
  (params (Count :type Integer))
  (bind _money (Variables|Default|GetMoney))
  (bind _returnvalue (- _money Count))
  (if (> Count 0)
    (if (>= _returnvalue 0)
      (Money|SetMoney _returnvalue)
      (LocalVariables|SetDone true)))
  (return (LocalVariables|GetDone)))

(fn GetMoney
  (return (Variables|Default|GetMoney)))