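; BP_Hand is the player's hand actor, which grabs, releases and throws other actors.
; Grab records each primitive component's physics and collision state, disables both and snaps the target to the hand; Release detaches it and reapplies that state.
; A looping timer, paused and unpaused on demand, builds clamped throw strength.
; Throw releases the item, applies an impulse along the owning BP_Player's camera direction to simulating components, then resets the charge.
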(event Custom|StartCharging
  (bind _chargingtimerhandle (Variables|Throw|GetChargingTimerHandle))
  (if (Utilities|Time|IsValidTimerHandle _chargingtimerhandle)
    (Utilities|Time|UnpauseTimerbyHandle _chargingtimerhandle)
    (Default|CallOnStartCharging)))

(event Custom|StopCharging
  (bind _chargingtimerhandle (Variables|Throw|GetChargingTimerHandle))
  (if (Utilities|Time|IsValidTimerHandle _chargingtimerhandle)
    (Utilities|Time|PauseTimerbyHandle _chargingtimerhandle)))

(event Custom|Charging
  (CallFunction|SetThrowStrenght (+ (Variables|Throw|GetCurrentThrowStrenght) (Variables|Throw|GetChargeStr))))

(event EventBeginPlay
  (Variables|Throw|SetChargeStr (/ (Variables|Throw|GetMaxThrowStrenght) (* (Variables|Throw|GetChargingTime) (Math|Conversions|ToFloat(Integer) (Variables|Throw|GetChargPerSec)))))
  (bind _returnvalue (Utilities|Time|SetTimerbyEvent (delegate Custom|Charging) (/ 1.0 (Math|Conversions|ToFloat(Integer) (Variables|Throw|GetChargPerSec))) true 0.1))
  (bind _output_get (Variables|Throw|SetChargingTimerHandle _returnvalue))
  (Utilities|Time|PauseTimerbyHandle _output_get))

(fn ConstructionScript)

(fn Grab
  (params (Target :type Actor%20Object%20Reference))
  (if (not (Variables|GrabbedActor|GetHasGrabbed))
    (for _array_element (Actor|GetComponentsByClass Target "/Script/Engine.PrimitiveComponent")
      (Utilities|Array|Add (Variables|GrabbedActor|GetGrabbedItemInfo) (Utilities|Struct|MakeF_GrabbedActor (Physics|IsSimulatingPhysics _array_element "None") (Collision|GetCollisionEnabled _array_element)))
      (Physics|SetSimulatePhysics _array_element false)
      (Collision|SetCollisionEnabled _array_element "NoCollision"))
    (Transformation|AttachActorToActor Target self "None" "SnapToTarget" "SnapToTarget" "SnapToTarget" true)
    (Variables|GrabbedActor|SetGrabbedActor Target)
    (Variables|GrabbedActor|SetHasGrabbed true)
    (Default|CallOnGrab)))

(fn Release
  (bind _grabbedactor (Variables|GrabbedActor|GetGrabbedActor))
  (if (Variables|GrabbedActor|GetHasGrabbed)
    (LocalVariables|SetRelActor (Variables|GrabbedActor|GetGrabbedActor))
    (Transformation|DetachFromActor _grabbedactor "KeepWorld" "KeepWorld" "KeepWorld")
    (for (_array_element _array_index) (Actor|GetComponentsByClass _grabbedactor "/Script/Engine.PrimitiveComponent")
      (Physics|SetSimulatePhysics _array_element (.simulate (Utilities|Array|Get(acopy) (Variables|GrabbedActor|GetGrabbedItemInfo) _array_index)))
      (Collision|SetCollisionEnabled _array_element (.collision (Utilities|Array|Get(acopy) (Variables|GrabbedActor|GetGrabbedItemInfo) _array_index)))))
  (Variables|GrabbedActor|SetHasGrabbed false)
  (Default|CallOnRelease)
  (return (LocalVariables|GetRelActor)))

(fn GetGrabbedActor
  (return (Variables|GrabbedActor|GetHasGrabbed) (Variables|GrabbedActor|GetGrabbedActor)))

(fn SetThrowStrenght
  (params (Strenght :type Float%20%28single-precision%29))
  (Variables|Throw|SetCurrentThrowStrenght (Math|Float|Clamp(Float) Strenght 0.0 (Variables|Throw|GetMaxThrowStrenght))))

(fn Throw
  (if (Variables|GrabbedActor|GetHasGrabbed)
    (bind _releasedactor (CallFunction|Release))
    (for _array_element (Actor|GetComponentsByClass _releasedactor "/Script/Engine.PrimitiveComponent")
      (if (Physics|IsSimulatingPhysics _array_element "None")
        (bind _asbp_player (Utilities|Casting|CastToBP_Player (Components|GetOwner)))
        (Physics|AddImpulse _array_element (* (Math|Vector|GetForwardVector (Variables|/Game/VTBMetaFive/GameLogic/Blueprints/Player/BP_Player.BP_Player_C|GetCamera _asbp_player)) (Variables|Throw|GetCurrentThrowStrenght)) "None" false)
        (CallFunction|StopCharging)
        (CallFunction|SetThrowStrenght 0.0)))
    (CallFunction|StopCharging)
    (CallFunction|SetThrowStrenght 0.0)))

(fn GetCurrentChargeNorm
  (return (Math|Float|MapRangeClamped (Variables|Throw|GetCurrentThrowStrenght) 0.0 (Variables|Throw|GetMaxThrowStrenght) 0.0 1.0)))