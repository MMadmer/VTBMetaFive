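; BP_Player is the player Blueprint, handling interaction with and grabbing of objects.
; On BeginPlay it spawns a BP_Hand actor, attaches it to the Hand component and announces it.
; Overlaps on the InteractionChecker sphere update a cached can-interact state, broadcasting changes when any overlapped actor is interactable or tagged "grab".
; TryInteract and TryGrab target via a camera-forward trace as long as the sphere's radius, messaging the target or passing grab-tagged actors to the hand.
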(event OnComponentBeginOverlap(InteractionChecker)
  (params (OverlappedComponent :type Primitive%20Component%20Object%20Reference) (OtherActor :type Actor%20Object%20Reference) (OtherComp :type Primitive%20Component%20Object%20Reference) (OtherBodyIndex :type Integer) (bFromSweep :type Boolean) (SweepResult :type Hit%20Result%20Structure%20%28by%20ref%29))
  (CallFunction|UpdateInteractions))

(event OnComponentEndOverlap(InteractionChecker)
  (params (OverlappedComponent :type Primitive%20Component%20Object%20Reference) (OtherActor :type Actor%20Object%20Reference) (OtherComp :type Primitive%20Component%20Object%20Reference) (OtherBodyIndex :type Integer))
  (CallFunction|UpdateInteractions))

(event EventBeginPlay
  (Hand|SpawnHand))

(fn ConstructionScript)

(fn UpdateInteractions
  (bind _array_element (Utilities|Array|ForEachLoopwithBreak (Collision|GetOverlappingActors (Variables|Default|GetInteractionChecker) 0 :!class /Script/Engine.PrimitiveComponent) :!label _label)
    (:LoopBody
      (bind _can (Class|BPIInteraction|CanInteract(Message) _array_element))
      (if (or _can (Actor|ActorHasTag _array_element "grab"))
        (LocalVariables|SetCan true)
        (goto _label Break)))
    (:Completed
      (if (Math|Boolean|Equal(Boolean) (LocalVariables|GetCan) (Variables|Default|GetCanInteract))
        _
        (else
          (Default|CallInteractionChanged (LocalVariables|GetCan))))
      (Variables|Default|SetCanInteract (LocalVariables|GetCan))
      (return))))

(fn GetCanInteract
  (return (Variables|Default|GetCanInteract)))

(fn SpawnHand
  (bind _returnvalue (Game|SpawnActorfromClass "/Game/VTBMetaFive/GameLogic/Blueprints/Player/BP_Hand.BP_Hand_C" (Transformation|GetWorldTransform (Variables|Default|GetHand)) "AlwaysSpawn" 0 0))
  (Variables|Default|SetPlayerHand _returnvalue)
  (Transformation|AttachComponentToComponent _returnvalue (Variables|Default|GetHand) "None" "SnapToTarget" "SnapToTarget" "KeepWorld" true)
  (Actor|SetOwner _returnvalue self)
  (Default|CallOnHandAdded _returnvalue))

(fn GetHand
  (return (Variables|Default|GetPlayerHand)))

(fn FindInterTarget
  (bind _camera (Variables|Default|GetCamera))
  (bind _desiredview (Class|CameraComponent|GetCameraView _camera 0.0))
  (bind _outhit (Collision|LineTraceByChannel (.location _desiredview) (+ (.location _desiredview) (* (Math|Vector|GetForwardVector _camera) (Variables|/Script/Engine.SphereComponent|GetSphereRadius (Variables|Default|GetInteractionChecker)))) "TraceTypeQuery1" false 0 "None"))
  (return (.HitActor (Collision|BreakHitResult _outhit))))

(fn TryInteract
  (bind _output_get (LocalVariables|SetTarget (CallFunction|FindInterTarget)))
  (Utilities|IsValid _output_get
    (:Is%20Valid
      (Class|BPIInteraction|Interact(Message) _output_get self)
      (CallFunction|UpdateInteractions))))

(fn TryGrab
  (bind _target (CallFunction|FindInterTarget))
  (bind _playerhand (Variables|Default|GetPlayerHand))
  (Utilities|IsValid _playerhand
    (:Is%20Valid
      (Utilities|IsValid _target
        (:Is%20Valid
          (bind _output_get (LocalVariables|SetTarget _target))
          (if (Actor|ActorHasTag _output_get "grab")
            (Default|Grab _playerhand (LocalVariables|GetTarget))))))))